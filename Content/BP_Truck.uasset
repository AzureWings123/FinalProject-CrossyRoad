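; BP_Truck is a moving truck hazard that ends the game when it hits BP_Player.
; Tick moves it along world Y, scaled by TruckSpeed and its forward vector's X, and randomly plays a horn at world origin.
; Three colliders each reshape or reset the player mesh's transform, such as squashing it, then display game over and destroy the truck.
; RandomizeTruck picks one of three truck meshes, but is not called here.
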(event OnComponentBeginOverlap(TruckCollider)
  (params (OverlappedComponent :type Primitive%20Component%20Object%20Reference) (OtherActor :type Actor%20Object%20Reference) (OtherComp :type Primitive%20Component%20Object%20Reference) (OtherBodyIndex :type Integer) (bFromSweep :type Boolean) (SweepResult :type Hit%20Result%20Structure%20%28by%20ref%29))
  (bind _asbp_player (Utilities|Casting|CastToBP_Player OtherActor))
  (Transformation|SetWorldTransform (Variables|/Game/BP_Player.BP_Player_C|GetStaticMesh _asbp_player) (Math|Transform|MakeTransform (- (Transformation|GetWorldLocation (Variables|/Script/Engine.Actor|GetRootComponent _asbp_player)) "0, 0,5.000000") "0, 0, 0" "0.500000,0.500000,0.100000") false false)
  (Default|DisplayGameOver _asbp_player)
  (Actor|DestroyActor))

(event OnComponentBeginOverlap(TruckCollision1)
  (params (OverlappedComponent :type Primitive%20Component%20Object%20Reference) (OtherActor :type Actor%20Object%20Reference) (OtherComp :type Primitive%20Component%20Object%20Reference) (OtherBodyIndex :type Integer) (bFromSweep :type Boolean) (SweepResult :type Hit%20Result%20Structure%20%28by%20ref%29))
  (bind _asbp_player (Utilities|Casting|CastToBP_Player OtherActor))
  (Transformation|SetWorldTransform (Variables|/Game/BP_Player.BP_Player_C|GetStaticMesh _asbp_player) (Math|Transform|MakeTransform (Transformation|GetWorldLocation (Variables|/Script/Engine.Actor|GetRootComponent _asbp_player)) "0, 0, 0" "0.100000,0.500000,0.500000") false false)
  (Default|DisplayGameOver _asbp_player)
  (Actor|DestroyActor))

(event OnComponentBeginOverlap(TruckCollision2)
  (params (OverlappedComponent :type Primitive%20Component%20Object%20Reference) (OtherActor :type Actor%20Object%20Reference) (OtherComp :type Primitive%20Component%20Object%20Reference) (OtherBodyIndex :type Integer) (bFromSweep :type Boolean) (SweepResult :type Hit%20Result%20Structure%20%28by%20ref%29))
  (bind _asbp_player (Utilities|Casting|CastToBP_Player OtherActor))
  (Transformation|SetWorldTransform (Variables|/Game/BP_Player.BP_Player_C|GetStaticMesh _asbp_player) (Math|Transform|MakeTransform "0, 0, 0" "0, 0, 0" "1,1,1") false false)
  (Default|DisplayGameOver _asbp_player)
  (Actor|DestroyActor))

(event EventBeginPlay)

(event Collision|EventActorBeginOverlap
  (params (OtherActor :type Actor%20Object%20Reference)))

(event EventTick
  (params (DeltaSeconds :type Float%20%28single-precision%29))
  (Transformation|AddActorWorldOffset (Math|Vector|MakeVector 0.0 (* (* DeltaSeconds (Variables|Default|GettruckSpeed)) (.x (Transformation|GetActorForwardVector))) 0.0))
  (if (== 5 (Math|Random|RandomInteger 400))
    (Audio|SpawnSoundatLocation "/Game/TruckHorn_Cue.TruckHorn_Cue" "0, 0, 0" "0, 0, 0" 1.0 1.0 0.0 0 0)))

(fn ConstructionScript)

(fn RandomizeTruck
  (Components|StaticMesh|SetStaticMesh (Variables|Default|GetTruckMesh) (Utilities|Select :Index (Math|Random|RandomIntegerinRange 0 2) :Option%200 "/Game/OilTanker.OilTanker" :Option%201 "/Game/PTruck.PTruck" :Option%202 "/Game/RTruck.RTruck")))