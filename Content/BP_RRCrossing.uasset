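; BP_RRCrossing is a railroad crossing signal that runs a repeating warning cycle of alternating lights and bell sounds.
; Tick counts frames through an idle wait, a slower flashing phase and a faster flashing phase, then turns both lights off and resets, so timing depends on frame rate.
; Each Warning call swaps LeftLight and RightLight intensity and plays RRBell_Cue at the world origin rather than the actor's location.
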(event EventBeginPlay)

(event Collision|EventActorBeginOverlap
  (params (OtherActor :type Actor%20Object%20Reference)))

(event EventTick
  (params (DeltaSeconds :type Float%20%28single-precision%29))
  (if (== (Variables|Default|Getcount) 0)
    (if (Variables|Default|Getwarning1)
      (if (Variables|Default|Getwarning2)
        (Rendering|Components|Light|SetIntensity (Variables|Default|GetRightLight) 0.0)
        (Rendering|Components|Light|SetIntensity (Variables|Default|GetLeftLight) 0.0)
        (Variables|Default|Setwarning1 false)
        (Variables|Default|Setwarning2 false)
        (Variables|Default|Setcount 150)
        (Variables|Default|SetwarningCount 0)
        (Variables|Default|Setcount2 20)
        (Variables|Default|Setwarning2Count 0)
        (Variables|Default|Setcount3 10)
        (elif (== 0 (Variables|Default|Getcount3))
          (CallFunction|Warning)
          (Math|Integer|IncrementInt (Variables|Default|Getwarning2Count)
            (:%20%20
              (Variables|Default|Setcount3 10)
              (if (== 10 (Variables|Default|Getwarning2Count))
                (Variables|Default|Setwarning2 true))))
          (else
            (Math|Integer|DecrementInt (Variables|Default|Getcount3)))))
      (elif (== (Variables|Default|Getcount2) 0)
        (CallFunction|Warning)
        (Math|Integer|IncrementInt (Variables|Default|GetwarningCount)
          (:%20%20
            (Variables|Default|Setcount2 20)
            (if (== 10 (Variables|Default|GetwarningCount))
              (Variables|Default|Setwarning1 true))))
        (else
          (Math|Integer|DecrementInt (Variables|Default|Getcount2)))))
    (else
      (Math|Integer|DecrementInt (Variables|Default|Getcount)))))

(fn ConstructionScript)

(fn Warning
  (if (== (Variables|/Script/Engine.LightComponentBase|GetIntensity (Variables|Default|GetLeftLight)) 0.0)
    (Rendering|Components|Light|SetIntensity (Variables|Default|GetLeftLight) 1e+04)
    (Rendering|Components|Light|SetIntensity (Variables|Default|GetRightLight) 0.0)
    (Audio|PlaySoundatLocation "/Game/RRBell_Cue.RRBell_Cue" "0, 0, 0" "0, 0, 0" 1.0 1.0 0.0 0 0 0)
    (else
      (Rendering|Components|Light|SetIntensity (Variables|Default|GetLeftLight) 0.0)
      (Rendering|Components|Light|SetIntensity (Variables|Default|GetRightLight) 1e+04)
      (Audio|PlaySoundatLocation "/Game/RRBell_Cue.RRBell_Cue" "0, 0, 0" "0, 0, 0" 1.0 1.0 0.0 0 0 0))))