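; BP_Car is a moving car hazard that ends the game when it hits BP_Player.
; Tick sweeps it along world Y, scaled by CarSpeed and forward-vector X, and occasionally honks at world origin.
; Three collision overlaps flatten the player's mesh along different axes, call DisplayGameOver and destroy the car.
; RandomizeCar picks one of four meshes and sizes CarCollision using separate random rolls, so size may mismatch mesh.
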(event OnComponentBeginOverlap(CarCollision)
  (params (OverlappedComponent :type Primitive%20Component%20Object%20Reference) (OtherActor :type Actor%20Object%20Reference) (OtherComp :type Primitive%20Component%20Object%20Reference) (OtherBodyIndex :type Integer) (bFromSweep :type Boolean) (SweepResult :type Hit%20Result%20Structure%20%28by%20ref%29))
  (bind _asbp_player (Utilities|Casting|CastToBP_Player OtherActor))
  (Transformation|SetWorldTransform (Variables|/Game/BP_Player.BP_Player_C|GetStaticMesh _asbp_player) (Math|Transform|MakeTransform (- (Transformation|GetWorldLocation (Variables|/Script/Engine.Actor|GetRootComponent _asbp_player)) "0, 0,5.000000") "0, 0, 0" "0.500000,0.500000,0.100000") false false)
  (Default|DisplayGameOver _asbp_player)
  (Actor|DestroyActor))

(event OnComponentBeginOverlap(CarCollision1)
  (params (OverlappedComponent :type Primitive%20Component%20Object%20Reference) (OtherActor :type Actor%20Object%20Reference) (OtherComp :type Primitive%20Component%20Object%20Reference) (OtherBodyIndex :type Integer) (bFromSweep :type Boolean) (SweepResult :type Hit%20Result%20Structure%20%28by%20ref%29))
  (bind _asbp_player (Utilities|Casting|CastToBP_Player OtherActor))
  (Transformation|SetWorldTransform (Variables|/Game/BP_Player.BP_Player_C|GetStaticMesh _asbp_player) (Math|Transform|MakeTransform (Transformation|GetWorldLocation (Variables|/Script/Engine.Actor|GetRootComponent _asbp_player)) "0,0.000000, 0" "0.100000,0.500000,0.500000") false false)
  (Default|DisplayGameOver _asbp_player)
  (Actor|DestroyActor))

(event OnComponentBeginOverlap(CarCollision2)
  (params (OverlappedComponent :type Primitive%20Component%20Object%20Reference) (OtherActor :type Actor%20Object%20Reference) (OtherComp :type Primitive%20Component%20Object%20Reference) (OtherBodyIndex :type Integer) (bFromSweep :type Boolean) (SweepResult :type Hit%20Result%20Structure%20%28by%20ref%29))
  (bind _asbp_player (Utilities|Casting|CastToBP_Player OtherActor))
  (Transformation|SetWorldTransform (Variables|/Game/BP_Player.BP_Player_C|GetStaticMesh _asbp_player) (Math|Transform|MakeTransform (Transformation|GetWorldLocation (Variables|/Script/Engine.Actor|GetRootComponent _asbp_player)) "0,0.000000, 0" "0.100000,0.500000,0.500000") false false)
  (Default|DisplayGameOver _asbp_player)
  (Actor|DestroyActor))

(event EventBeginPlay)

(event Collision|EventActorBeginOverlap
  (params (OtherActor :type Actor%20Object%20Reference)))

(event EventTick
  (params (DeltaSeconds :type Float%20%28single-precision%29))
  (Transformation|AddActorWorldOffset (Math|Vector|MakeVector 0.0 (* (* DeltaSeconds (Variables|Default|GetcarSpeed)) (.x (Transformation|GetActorForwardVector))) 0.0) true)
  (if (== 5 (Math|Random|RandomInteger 350))
    (Audio|SpawnSoundatLocation "/Game/CarHorn_Cue.CarHorn_Cue" "0, 0, 0" "0, 0, 0" 1.0 1.0 0.0 0 0)))

(fn ConstructionScript)

(fn RandomizeCar
  (bind _returnvalue (Math|Random|RandomIntegerinRange 0 3))
  (Components|StaticMesh|SetStaticMesh (Variables|Default|GetStaticMesh) (Utilities|Select :Index _returnvalue :Option%200 "/Game/BCar.BCar" :Option%201 "/Game/GCar.GCar" :Option%202 "/Game/OCar.OCar" :Option%203 "/Game/PCar.PCar"))
  (if (or (== _returnvalue 0) (== 3 _returnvalue))
    (Components|Box|SetBoxExtent (Variables|Default|GetCarCollision) "32.000000,100.000000,40.000000" true)
    (else
      (Components|Box|SetBoxExtent (Variables|Default|GetCarCollision) "32.000000,70.000000,32.000000" true))))