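; BP_Train is a moving train hazard that sounds a horn at spawn and ends the game when it hits BP_Player.
; Tick moves it along world Y, scaled by TrainSpeed and its forward vector's X.
; Three trigger boxes squash the player's mesh flat or thin, show game over, then destroy the train.
; RandomizeTrain, not called here, picks mesh and main box length using separate random rolls, so they can mismatch.
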(event OnComponentBeginOverlap(TrainBox)
  (params (OverlappedComponent :type Primitive%20Component%20Object%20Reference) (OtherActor :type Actor%20Object%20Reference) (OtherComp :type Primitive%20Component%20Object%20Reference) (OtherBodyIndex :type Integer) (bFromSweep :type Boolean) (SweepResult :type Hit%20Result%20Structure%20%28by%20ref%29))
  (bind _asbp_player (Utilities|Casting|CastToBP_Player OtherActor))
  (Transformation|SetWorldTransform (Variables|/Game/BP_Player.BP_Player_C|GetStaticMesh _asbp_player) (Math|Transform|MakeTransform (- (Transformation|GetWorldLocation (Variables|/Script/Engine.Actor|GetRootComponent _asbp_player)) "0, 0,5.000000") "0, 0, 0" "0.500000,0.500000,0.100000") false false)
  (Default|DisplayGameOver _asbp_player)
  (Actor|DestroyActor))

(event OnComponentBeginOverlap(TrainBox1)
  (params (OverlappedComponent :type Primitive%20Component%20Object%20Reference) (OtherActor :type Actor%20Object%20Reference) (OtherComp :type Primitive%20Component%20Object%20Reference) (OtherBodyIndex :type Integer) (bFromSweep :type Boolean) (SweepResult :type Hit%20Result%20Structure%20%28by%20ref%29))
  (bind _asbp_player (Utilities|Casting|CastToBP_Player OtherActor))
  (Transformation|SetWorldTransform (Variables|/Game/BP_Player.BP_Player_C|GetStaticMesh _asbp_player) (Math|Transform|MakeTransform (Transformation|GetWorldLocation (Variables|/Script/Engine.Actor|GetRootComponent _asbp_player)) "0, 0, 0" "0.100000,0.500000,0.500000") false false)
  (Default|DisplayGameOver _asbp_player)
  (Actor|DestroyActor))

(event OnComponentBeginOverlap(TrainBox2)
  (params (OverlappedComponent :type Primitive%20Component%20Object%20Reference) (OtherActor :type Actor%20Object%20Reference) (OtherComp :type Primitive%20Component%20Object%20Reference) (OtherBodyIndex :type Integer) (bFromSweep :type Boolean) (SweepResult :type Hit%20Result%20Structure%20%28by%20ref%29))
  (bind _asbp_player (Utilities|Casting|CastToBP_Player OtherActor))
  (Transformation|SetWorldTransform (Variables|/Game/BP_Player.BP_Player_C|GetStaticMesh _asbp_player) (Math|Transform|MakeTransform (Transformation|GetWorldLocation (Variables|/Script/Engine.Actor|GetRootComponent _asbp_player)) "0, 0, 0" "0.100000,0.500000,0.500000") false false)
  (Default|DisplayGameOver _asbp_player)
  (Actor|DestroyActor))

(event EventBeginPlay
  (Audio|PlaySoundatLocation "/Game/TrainHorn_Cue.TrainHorn_Cue" "0, 0, 0" "0, 0, 0" 1.0 1.0 0.0 0 0 0))

(event Collision|EventActorBeginOverlap
  (params (OtherActor :type Actor%20Object%20Reference)))

(event EventTick
  (params (DeltaSeconds :type Float%20%28single-precision%29))
  (Transformation|AddActorWorldOffset (Math|Vector|MakeVector 0.0 (* (* DeltaSeconds (Variables|Default|GettrainSpeed)) (.x (Transformation|GetActorForwardVector))) 0.0)))

(fn ConstructionScript)

(fn RandomizeTrain
  (bind _returnvalue (Math|Random|RandomIntegerinRange 0 1))
  (Components|StaticMesh|SetStaticMesh (Variables|Default|GetStaticMesh) (Utilities|Select :Index _returnvalue :Option%200 "/Game/5Train.5Train" :Option%201 "/Game/6Train.6Train"))
  (if (== 0 _returnvalue)
    (Components|Box|SetBoxExtent (Variables|Default|GetTrainBox) "41.000000,800.000000,100.000000" true)
    (else
      (Components|Box|SetBoxExtent (Variables|Default|GetTrainBox) "41.000000,930.000000,100.000000" true))))