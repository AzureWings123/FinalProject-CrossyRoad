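; BP_Lane is one randomized lane of grass, road, river or railway in a Crossy Road-style game.
; RandomizeLane picks type, mesh and direction, alternating grass for early lanes, and places obstacles or coins.
; Tick spawns vehicles, trains, logs or lilies by type, using random rolls or Delays.
; Overlaps remove cars at triggers, end the game in rivers, and make LaneSpawner add a lane as this one destroys itself.
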(event OnComponentBeginOverlap(TriggerZone)
  (params (OverlappedComponent :type Primitive%20Component%20Object%20Reference) (OtherActor :type Actor%20Object%20Reference) (OtherComp :type Primitive%20Component%20Object%20Reference) (OtherBodyIndex :type Integer) (bFromSweep :type Boolean) (SweepResult :type Hit%20Result%20Structure%20%28by%20ref%29))
  (Utilities|Casting|CastToBP_Player OtherActor)
  (Default|SpawnLaneatSpawnPoint (Variables|Default|GetLaneSpawner))
  (Actor|DestroyActor))

(event OnComponentBeginOverlap(CarTrigger1)
  (params (OverlappedComponent :type Primitive%20Component%20Object%20Reference) (OtherActor :type Actor%20Object%20Reference) (OtherComp :type Primitive%20Component%20Object%20Reference) (OtherBodyIndex :type Integer) (bFromSweep :type Boolean) (SweepResult :type Hit%20Result%20Structure%20%28by%20ref%29))
  (bind _asbp_car (Utilities|Casting|CastToBP_Car OtherActor))
  (Actor|DestroyActor _asbp_car))

(event OnComponentBeginOverlap(CarTrigger2)
  (params (OverlappedComponent :type Primitive%20Component%20Object%20Reference) (OtherActor :type Actor%20Object%20Reference) (OtherComp :type Primitive%20Component%20Object%20Reference) (OtherBodyIndex :type Integer) (bFromSweep :type Boolean) (SweepResult :type Hit%20Result%20Structure%20%28by%20ref%29))
  (bind _asbp_car (Utilities|Casting|CastToBP_Car OtherActor))
  (Actor|DestroyActor _asbp_car))

(event OnComponentBeginOverlap(LaneHitBox)
  (params (OverlappedComponent :type Primitive%20Component%20Object%20Reference) (OtherActor :type Actor%20Object%20Reference) (OtherComp :type Primitive%20Component%20Object%20Reference) (OtherBodyIndex :type Integer) (bFromSweep :type Boolean) (SweepResult :type Hit%20Result%20Structure%20%28by%20ref%29))
  (bind _asbp_player (Utilities|Casting|CastToBP_Player OtherActor))
  ;[1 1 1] Prep for game over condition: river
  (if (== (Variables|Default|GetLaneType) 4)
    (Development|PrintString "You are not a duck")
    (Effects|SpawnEmitteratLocation "/Game/PS_Splash.PS_Splash" (Transformation|GetActorLocation _asbp_player))
    (Audio|PlaySoundatLocation "/Game/Splash_Cue.Splash_Cue" "0, 0, 0" "0, 0, 0" 1.0 1.0 0.0 0 0 0)
    (Default|DisplayGameOver _asbp_player)))

(event EventBeginPlay)

(event Collision|EventActorBeginOverlap
  (params (OtherActor :type Actor%20Object%20Reference)))

(event EventTick
  (params (DeltaSeconds :type Float%20%28single-precision%29))
  (bind _self self)
  (bind _self_2 self)
  (bind _self_3 self)
  (bind _carspawn2 (Variables|Default|GetCarSpawn2 _self_2))
  (bind _carspawn1 (Variables|Default|GetCarSpawn1 _self))
  (bind _carspawn2_2 (Variables|Default|GetCarSpawn2 _self))
  (bind _carspawn1_2 (Variables|Default|GetCarSpawn1 _self_2))
  (bind _returnvalue (Transformation|GetWorldLocation _carspawn2))
  (bind _returnvalue_2 (Transformation|GetWorldLocation _carspawn1_2))
  (bind _returnvalue_3 (Transformation|GetWorldLocation _carspawn1))
  (bind _returnvalue_4 (Transformation|GetWorldLocation _carspawn2_2))
  ;[1 1 1] Spawn a Car or Truck
  (if (or (== (Variables|Default|GetLaneType) 2) (== (Variables|Default|GetLaneType) 3))
    (if (== 10 (Math|Random|RandomIntegerinRange 0 200))
      (if (== (Math|Random|RandomIntegerinRange 0 1) 0)
        (if (Variables|Default|GetGoingLeftToRight)
          (Utilities|FlowControl|Delay 1.0)
          (if (Math|Random|RandomBool)
            (CallFunction|SpawnPolice _returnvalue_2)
            (else
              (CallFunction|SpawnCar _returnvalue_2)))
          (else
            (Utilities|FlowControl|Delay 1.0)
            (if (Math|Random|RandomBool)
              (CallFunction|SpawnPolice _returnvalue)
              (else
                (CallFunction|SpawnCar _returnvalue)))))
        (elif (Variables|Default|GetGoingLeftToRight)
          (Utilities|FlowControl|Delay 1.0)
          (CallFunction|SpawnTruck _returnvalue_2)
          (else
            (Utilities|FlowControl|Delay 1.0)
            (CallFunction|SpawnTruck _returnvalue)))))
    (else
      ;[1 1 1] Spawn a Train
      (if (== (Variables|Default|GetLaneType) 5)
        (if (Variables|Default|GetGoingLeftToRight)
          (Utilities|FlowControl|Delay 12.6)
          (CallFunction|SpawnTrain (Transformation|GetWorldLocation (Variables|Default|GetCarSpawn1 _self_3)))
          (else
            (Utilities|FlowControl|Delay 12.6)
            (CallFunction|SpawnTrain (Transformation|GetWorldLocation (Variables|Default|GetCarSpawn2 _self_3)))))
        (elif (== (Variables|Default|GetLaneType) 4)
          (if (== 10 (Math|Random|RandomIntegerinRange 0 200))
            (if (Variables|Default|GetGoingLeftToRight)
              (if (Variables|Default|GetLilyOrLog)
                (CallFunction|SpawnLily _returnvalue_3)
                (else
                  (CallFunction|SpawnLog _returnvalue_3)))
              (elif (Variables|Default|GetLilyOrLog)
                (CallFunction|SpawnLily _returnvalue_4)
                (else
                  (CallFunction|SpawnLog _returnvalue_4))))))))))

(fn ConstructionScript)

(fn RandomizeLane
  (params (HoldingCount :type Integer))
  (bind _spawnobs2 (Variables|Default|GetSpawnObs2))
  (bind _spawnobs3 (Variables|Default|GetSpawnObs3))
  (bind _spawnobs4 (Variables|Default|GetSpawnObs4))
  (bind _spawnobs5 (Variables|Default|GetSpawnObs5))
  (bind _spawnobs6 (Variables|Default|GetSpawnObs6))
  (bind _spawnobs (Variables|Default|GetSpawnObs))
  (bind _returnvalue (Transformation|GetWorldLocation _spawnobs2))
  (bind _returnvalue_2 (Transformation|GetWorldLocation _spawnobs))
  (bind _returnvalue_3 (Transformation|GetWorldLocation _spawnobs6))
  (bind _returnvalue_4 (Transformation|GetWorldLocation _spawnobs5))
  (bind _returnvalue_5 (Transformation|GetWorldLocation _spawnobs4))
  (bind _returnvalue_6 (Transformation|GetWorldLocation _spawnobs3))
  (if (< HoldingCount 12)
    ;[1 1 1] Initial 10 alt grass lanes
    (bind _output_get (Variables|Default|SetLaneType (Math|Integer|%(Integer) HoldingCount 2)))
    (Components|StaticMesh|SetStaticMesh (Variables|Default|GetStaticMesh) (Utilities|Select :Index _output_get :Option%200 "/Game/LGrass.LGrass" :Option%201 "/Game/DGrass.DGrass"))
    (Variables|Default|SetGoingLeftToRight (Math|Random|RandomBool))
    (else
      (bind _output_get_2 (Variables|Default|SetLaneType (Math|Random|RandomIntegerinRange 0 5)))
      (Components|StaticMesh|SetStaticMesh (Variables|Default|GetStaticMesh) (Utilities|Select :Index _output_get_2 :Option%200 "/Game/LGrass.LGrass" :Option%201 "/Game/DGrass.DGrass" :Option%202 "/Game/Highway.Highway" :Option%203 "/Game/UHighway.UHighway" :Option%204 "/Game/River.River" :Option%205 "/Game/RRoad.RRoad"))
      (Variables|Default|SetGoingLeftToRight (Math|Random|RandomBool))
      (Variables|Default|SetLilyOrLog (Math|Random|RandomBool))))
  (if (or (== 1 (Variables|Default|GetLaneType)) (== 0 (Variables|Default|GetLaneType)))
    (Game|SpawnActorfromClass "/Game/BP_LTree.BP_LTree_C" (Math|Transform|MakeTransform (Transformation|GetWorldLocation (Variables|Default|GetEndTree1)) "0, 0, 0" "1,1,1") "Undefined" 0 0)
    (Game|SpawnActorfromClass "/Game/BP_LTree.BP_LTree_C" (Math|Transform|MakeTransform (Transformation|GetWorldLocation (Variables|Default|GetEndTree2)) "0, 0, 0" "1,1,1") "Undefined" 0 0)
    (CallFunction|SpawnObstacleorCoin _returnvalue_2)
    (CallFunction|SpawnObstacleorCoin _returnvalue)
    (CallFunction|SpawnObstacleorCoin _returnvalue_6)
    (CallFunction|SpawnObstacleorCoin _returnvalue_5)
    (CallFunction|SpawnObstacleorCoin _returnvalue_4)
    (CallFunction|SpawnObstacleorCoin _returnvalue_3)
    (elif (Math|Random|RandomBool)
      (Game|SpawnActorfromClass "/Game/BP_Coin.BP_Coin_C" (Math|Transform|MakeTransform _returnvalue_2 "0, 0, 0" "1,1,1") "Undefined" 0 0)
      (if (Math|Random|RandomBool)
        (Game|SpawnActorfromClass "/Game/BP_Coin.BP_Coin_C" (Math|Transform|MakeTransform _returnvalue "0, 0, 0" "1,1,1") "Undefined" 0 0)
        (if (Math|Random|RandomBool)
          (Game|SpawnActorfromClass "/Game/BP_Coin.BP_Coin_C" (Math|Transform|MakeTransform _returnvalue_6 "0, 0, 0" "1,1,1") "Undefined" 0 0)
          (if (Math|Random|RandomBool)
            (Game|SpawnActorfromClass "/Game/BP_Coin.BP_Coin_C" (Math|Transform|MakeTransform _returnvalue_5 "0, 0, 0" "1,1,1") "Undefined" 0 0)
            (if (Math|Random|RandomBool)
              (Game|SpawnActorfromClass "/Game/BP_Coin.BP_Coin_C" (Math|Transform|MakeTransform _returnvalue_4 "0, 0, 0" "1,1,1") "Undefined" 0 0)
              (if (Math|Random|RandomBool)
                (Game|SpawnActorfromClass "/Game/BP_Coin.BP_Coin_C" (Math|Transform|MakeTransform _returnvalue_3 "0, 0, 0" "1,1,1") "Undefined" 0 0)))))))))

(fn SpawnCar
  (params (SpawnLocation :type Vector))
  (bind _returnvalue (+ SpawnLocation "-4.000000, 0,-18.000000"))
  (if (Variables|Default|GetGoingLeftToRight)
    (bind _returnvalue_2 (Game|SpawnActorfromClass "/Game/BP_Car.BP_Car_C" (Math|Transform|MakeTransform _returnvalue "0,180.000000, 0" "1,1,1") "Undefined" 0 0))
    (Default|RandomizeCar _returnvalue_2)
    (else
      (bind _returnvalue_3 (Game|SpawnActorfromClass "/Game/BP_Car.BP_Car_C" (Math|Transform|MakeTransform _returnvalue "0, 0, 0" "1,1,1") "Undefined" 0 0))
      (Default|RandomizeCar _returnvalue_3))))

(fn SpawnTrain
  (params (SpawnLocation :type Vector))
  (bind _returnvalue (+ SpawnLocation "-20.000000,-100.000000,8.000000"))
  (if (Variables|Default|GetGoingLeftToRight)
    (bind _returnvalue_2 (Game|SpawnActorfromClass "/Game/BP_Train.BP_Train_C" (Math|Transform|MakeTransform _returnvalue "0,180.000000, 0" "1,1,1") "Undefined" 0 0))
    (Default|RandomizeTrain _returnvalue_2)
    (else
      (bind _returnvalue_3 (Game|SpawnActorfromClass "/Game/BP_Train.BP_Train_C" (Math|Transform|MakeTransform _returnvalue "0, 0, 0" "1,1,1") "Undefined" 0 0))
      (Default|RandomizeTrain _returnvalue_3))))

(fn SpawnTruck
  (params (TruckSpawnLocation :type Vector))
  (bind _returnvalue (+ TruckSpawnLocation "-4.000000,0.000000,-18.000000"))
  (if (Variables|Default|GetGoingLeftToRight)
    (bind _returnvalue_2 (Game|SpawnActorfromClass "/Game/BP_Truck.BP_Truck_C" (Math|Transform|MakeTransform _returnvalue "0,180.000000, 0" "1,1,1") "Undefined" 0 0))
    (Default|RandomizeTruck _returnvalue_2)
    (else
      (bind _returnvalue_3 (Game|SpawnActorfromClass "/Game/BP_Truck.BP_Truck_C" (Math|Transform|MakeTransform _returnvalue "0, 0, 0" "1,1,1") "Undefined" 0 0))
      (Default|RandomizeTruck _returnvalue_3))))

(fn SpawnLily
  (params (LilySpawnLocation :type Vector))
  (bind _returnvalue (+ LilySpawnLocation "-20.000000, 0,-18.000000"))
  (if (Variables|Default|GetGoingLeftToRight)
    (Game|SpawnActorfromClass "/Game/BP_Lily.BP_Lily_C" (Math|Transform|MakeTransform _returnvalue "0,180.000000, 0" "1,1,1") "Undefined" 0 0)
    (else
      (Game|SpawnActorfromClass "/Game/BP_Lily.BP_Lily_C" (Math|Transform|MakeTransform _returnvalue "0, 0, 0" "1,1,1") "Undefined" 0 0))))

(fn SpawnLog
  (params (LogSpawnLocation :type Vector))
  (bind _returnvalue (+ LogSpawnLocation "-20.000000, 0,0.000000"))
  (if (Variables|Default|GetGoingLeftToRight)
    (bind _returnvalue_2 (Game|SpawnActorfromClass "/Game/BP_Log.BP_Log_C" (Math|Transform|MakeTransform _returnvalue "0,180.000000, 0" "1,1,1") "Undefined" 0 0))
    (Default|RandomizeLog _returnvalue_2)
    (else
      (bind _returnvalue_3 (Game|SpawnActorfromClass "/Game/BP_Log.BP_Log_C" (Math|Transform|MakeTransform _returnvalue "0, 0, 0" "1,1,1") "Undefined" 0 0))
      (Default|RandomizeLog _returnvalue_3))))

(fn SpawnPolice
  (params (spawnLocation :type Vector))
  (if (Variables|Default|GetGoingLeftToRight)
    (Game|SpawnActorfromClass "/Game/BP_Police.BP_Police_C" (Math|Transform|MakeTransform spawnLocation "0,180.000000, 0" "1,1,1") "Undefined" 0 0)
    (else
      (Game|SpawnActorfromClass "/Game/BP_Police.BP_Police_C" (Math|Transform|MakeTransform spawnLocation "0, 0, 0" "1,1,1") "Undefined" 0 0))))

(fn SpawnObstacleorCoin
  (params (Location :type Vector))
  (if (Math|Random|RandomBool)
    (Game|SpawnActorfromClass (Utilities|Select :Index (Math|Random|RandomIntegerinRange 0 6) :Option%200 "/Game/BP_LTree.BP_LTree_C" :Option%201 "/Game/BP_MTree.BP_MTree_C" :Option%202 "/Game/BP_STree.BP_STree_C" :Option%203 "/Game/BP_LRock.BP_LRock_C" :Option%204 "/Game/BP_MRock.BP_MRock_C" :Option%205 "/Game/BP_SRock.BP_SRock_C" :Option%206 "/Game/BP_Coin.BP_Coin_C") (Math|Transform|MakeTransform Location "0, 0, 0" "1,1,1") "Undefined" 0 0)))