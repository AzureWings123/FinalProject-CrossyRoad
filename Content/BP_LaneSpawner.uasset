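; BP_LaneSpawner builds the chain of BP_Lane actors and tracks the lane count as the step score and high score.
; On BeginPlay it clears existing lanes, spawns an initial run ahead of the player, then creates the HUD.
; Each new lane attaches at the newest lane's SpawnPoint and randomizes its type from a capped counter.
; Railroad crossing signals spawn only within the new-high-score branch, for railroad lanes.
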(event EventBeginPlay
  (CallFunction|SpawnInitialLanes)
  (bind _returnvalue (UserInterface|CreateWidget "/Game/WBP_HUD.WBP_HUD_C"))
  (UserInterface|Viewport|AddtoViewport _returnvalue 0)
  (Variables|/Game/WBP_HUD.WBP_HUD_C|SetLanes _returnvalue self)
  (bind _output_get (Variables|Default|SetHudWidget _returnvalue))
  (Default|UpdateStepText _output_get))

(event Collision|EventActorBeginOverlap
  (params (OtherActor :type Actor%20Object%20Reference)))

(event EventTick
  (params (DeltaSeconds :type Float%20%28single-precision%29)))

(fn ConstructionScript)

(fn SpawnLane
  (params (SpawnLocation :type Vector))
  (bind _lanesspawned (Variables|Default|GetLanesSpawned))
  (bind _hudwidget (Variables|Default|GetHudWidget))
  (if (!= 12 (Variables|Default|GetTypeCounter))
    (Math|Integer|IncrementInt (Variables|Default|GetTypeCounter)
      (:%20%20
        _)))
  (bind _returnvalue (Game|SpawnActorfromClass "/Game/BP_Lane.BP_Lane_C" (Math|Transform|MakeTransform SpawnLocation "0, 0, 0" "1,1,1") "Undefined" 0 0))
  (bind _output_get (Variables|Default|SetNewestLane _returnvalue))
  (Variables|/Game/BP_Lane.BP_Lane_C|SetLaneSpawner _output_get self)
  (Default|RandomizeLane _output_get (Variables|Default|GetTypeCounter))
  (Math|Integer|IncrementInt _lanesspawned
    (:%20%20
      (Utilities|IsValid _hudwidget
        (:Is%20Valid
          (Default|UpdateStepText _hudwidget)
          (if (> _lanesspawned (Variables|Default|GetLaneHighScore))
            (Variables|Default|SetLaneHighScore _lanesspawned)
            (Default|UpdateStepHighScore _hudwidget)
            ;[1 1 1] If railroad, spawn in the signal too
            (if (== (Variables|/Game/BP_Lane.BP_Lane_C|GetLaneType (Variables|Default|GetNewestLane)) 5)
              (bind _returnvalue_2 (Game|SpawnActorfromClass "/Game/BP_RRCrossing.BP_RRCrossing_C" (Math|Transform|MakeTransform (Transformation|GetWorldLocation (Variables|/Game/BP_Lane.BP_Lane_C|GetRRCrossSpawnPoint (Variables|Default|GetNewestLane))) "0,-90.000000, 0" "1,1,1") "Undefined" 0 0))
              (Variables|Default|SetRRCross _returnvalue_2))))))))

(fn SpawnLaneatSpawnPoint
  (CallFunction|SpawnLane (Transformation|GetWorldLocation (Variables|/Game/BP_Lane.BP_Lane_C|GetSpawnPoint (Variables|Default|GetNewestLane)))))

(fn SpawnInitialLanes
  (Utilities|FlowControl|Sequence
    (:then_0
      (bind _outactors (Actor|GetAllActorsOfClass "/Game/BP_Lane.BP_Lane_C"))
      (for _array_element _outactors
        (Actor|DestroyActor _array_element)
        (Variables|Default|SetLanesSpawned -11)
        (Variables|Default|SetTypeCounter 0)))
    (:then_1
      (for _index (range 0 10)
        (Utilities|IsValid (Variables|Default|GetNewestLane)
          (:Is%20Valid
            (CallFunction|SpawnLaneatSpawnPoint))
          (:Is%20Not%20Valid
            (CallFunction|SpawnLane (+ (Transformation|GetActorLocation (Game|Player|GetPlayerPawn 0)) "380.000000, 0,-80.000000"))))))))