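; BP_Log is a moving log that reacts to the player entering or leaving its box.
; Tick slides it along world Y at LogSpeed scaled by the X of its forward vector.
; LogBox begin and end overlaps with BP_Player both play Log_Cue at the world origin.
; RandomizeLog picks one of two meshes and one of two box lengths using separate random rolls, and is not called within this Blueprint.
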(event OnComponentBeginOverlap(LogBox)
  (params (OverlappedComponent :type Primitive%20Component%20Object%20Reference) (OtherActor :type Actor%20Object%20Reference) (OtherComp :type Primitive%20Component%20Object%20Reference) (OtherBodyIndex :type Integer) (bFromSweep :type Boolean) (SweepResult :type Hit%20Result%20Structure%20%28by%20ref%29))
  (Utilities|Casting|CastToBP_Player OtherActor)
  (Audio|SpawnSoundatLocation "/Game/Log_Cue.Log_Cue" "0, 0, 0" "0, 0, 0" 1.0 1.0 0.0 0 0))

(event OnComponentEndOverlap(LogBox)
  (params (OverlappedComponent :type Primitive%20Component%20Object%20Reference) (OtherActor :type Actor%20Object%20Reference) (OtherComp :type Primitive%20Component%20Object%20Reference) (OtherBodyIndex :type Integer))
  (Utilities|Casting|CastToBP_Player OtherActor)
  (Audio|SpawnSoundatLocation "/Game/Log_Cue.Log_Cue" "0, 0, 0" "0, 0, 0" 1.0 1.0 0.0 0 0))

(event EventBeginPlay)

(event Collision|EventActorBeginOverlap
  (params (OtherActor :type Actor%20Object%20Reference)))

(event EventTick
  (params (DeltaSeconds :type Float%20%28single-precision%29))
  (Transformation|AddActorWorldOffset (Math|Vector|MakeVector 0.0 (* (* DeltaSeconds (Variables|Default|GetlogSpeed)) (.x (Transformation|GetActorForwardVector))) 0.0)))

(fn ConstructionScript)

(fn RandomizeLog
  (bind _returnvalue (Math|Random|RandomIntegerinRange 0 1))
  (Components|StaticMesh|SetStaticMesh (Variables|Default|GetLogMesh) (Utilities|Select :Index _returnvalue :Option%200 "/Game/BLog.BLog" :Option%201 "/Game/SLog.SLog"))
  (if (== 1 _returnvalue)
    (Components|Box|SetBoxExtent (Variables|Default|GetLogBox) "35.000000,75.000000,45.000000" true)
    (else
      (Components|Box|SetBoxExtent (Variables|Default|GetLogBox) "35.000000,100.000000,45.000000" true))))