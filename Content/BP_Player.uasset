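; Player character for a Crossy Road-style hopper, with coin HUD and game-over screen.
; Hop inputs squash and turn the mesh on press, then launch the character with a cluck on release.
; Tick drifts the camera and counts idle frames, playing periodic caws, then spawning an eagle and triggering game over; any hop press resets the timer.
; Restart destroys obstacle, vehicle and coin actors and resets HUD, input and mesh.
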(event EventBeginPlay
  (bind _returnvalue (UserInterface|CreateWidget "/Game/WBP_HUD.WBP_HUD_C"))
  (UserInterface|Viewport|AddtoViewport _returnvalue 0)
  (bind _returnvalue_2 (UserInterface|CreateWidget "/Game/WBP_GameOver.WBP_GameOver_C"))
  (Variables|Default|SetRestartHUD _returnvalue_2)
  (Variables|/Game/WBP_HUD.WBP_HUD_C|SetCoin _returnvalue self)
  (bind _output_get (Variables|Default|SetCoinHUD _returnvalue))
  (Default|UpdateCoinText _output_get))

(event Collision|EventActorBeginOverlap
  (params (OtherActor :type Actor%20Object%20Reference)))

(event EventTick
  (params (DeltaSeconds :type Float%20%28single-precision%29))
  (bind _waitforeagle (Variables|Default|GetwaitForEagle))
  (Transformation|AddWorldOffset (Variables|Default|GetCamera) "-0.200000, 0, 0" false false)
  (bind _result (Math|Float|IncrementFloat (Variables|Default|GeteagleTimer))
    (:%20%20
      (if (== _result 5e+02)
        (CallFunction|SpawnEagle (Transformation|GetWorldLocation (Variables|Default|GetEagleSpawn)))
        (elif (> _result 501.0)
          (Math|Integer|IncrementInt _waitforeagle
            (:%20%20
              (if (== 50 _waitforeagle)
                (CallFunction|DisplayGameOver))))
          (else
            (Math|Float|IncrementFloat (Variables|Default|GetcawCounter)
              (:%20%20
                (if (== 2.5e+02 (Variables|Default|GetcawCounter))
                  (Audio|PlaySoundatLocation "/Game/Caw_Cue.Caw_Cue" "0, 0, 0" "0, 0, 0" 1.0 1.0 0.0 0 0 0)
                  (Variables|Default|SetcawCounter 0.0))))))))))

(event Input|ActionEvents|InputActionHopDown
  (params (Key :type Key%20Structure :default "None"))
  (bind _staticmesh (Variables|Default|GetStaticMesh))
  ;[1 1 1] Down Movement
  (:Pressed
    (Transformation|SetWorldTransform _staticmesh (Math|Transform|MakeTransform (Transformation|GetActorLocation) "0,90.000000, 0" "0.500000,0.500000,0.250000") false false)
    (Variables|Default|SeteagleTimer 0.0))
  (:Released
    (Transformation|SetWorldScale3D _staticmesh "0.500000,0.500000,0.500000")
    (Character|LaunchCharacter "154.500000, 0,250.000000" false false)
    (Audio|PlaySoundatLocation "/Game/Cluck_Cue.Cluck_Cue" "0, 0, 0" "0, 0, 0" 1.0 1.0 0.0 0 0 0)
    (Transformation|AddWorldOffset (Variables|Default|GetCamera) "0.100000, 0, 0" false false)))

(event Input|ActionEvents|InputActionHopLeft
  (params (Key :type Key%20Structure :default "None"))
  (bind _staticmesh (Variables|Default|GetStaticMesh))
  ;[1 1 1] Left Movement
  (:Pressed
    (Transformation|SetWorldTransform _staticmesh (Math|Transform|MakeTransform (Transformation|GetActorLocation) "0,180.000000, 0" "0.500000,0.500000,0.250000") false false)
    (Variables|Default|SeteagleTimer 0.0))
  (:Released
    (Transformation|SetWorldScale3D _staticmesh "0.500000,0.500000,0.500000")
    (Character|LaunchCharacter "0.000000,160.000000,250.000000" false false)
    (Audio|PlaySoundatLocation "/Game/Cluck_Cue.Cluck_Cue" "0, 0, 0" "0, 0, 0" 1.0 1.0 0.0 0 0 0)))

(event Input|ActionEvents|InputActionHopRight
  (params (Key :type Key%20Structure :default "None"))
  (bind _staticmesh (Variables|Default|GetStaticMesh))
  ;[1 1 1] Right Movement
  (:Pressed
    (Transformation|SetWorldTransform _staticmesh (Math|Transform|MakeTransform (Transformation|GetActorLocation) "0, 0, 0" "0.500000,0.500000,0.250000") false false)
    (Variables|Default|SeteagleTimer 0.0))
  (:Released
    (Transformation|SetWorldScale3D _staticmesh "0.500000,0.500000,0.500000")
    (Character|LaunchCharacter "0.000000,-160.000000,250.000000" false false)
    (Audio|PlaySoundatLocation "/Game/Cluck_Cue.Cluck_Cue" "0, 0, 0" "0, 0, 0" 1.0 1.0 0.0 0 0 0)))

(event Input|ActionEvents|InputActionHopUp
  (params (Key :type Key%20Structure :default "None"))
  (bind _staticmesh (Variables|Default|GetStaticMesh))
  ;[1 1 1] Up Movement
  (:Pressed
    (Transformation|SetWorldTransform _staticmesh (Math|Transform|MakeTransform (Transformation|GetActorLocation) "0,270.000000, 0" "0.500000,0.500000,0.250000") false false)
    (Variables|Default|SeteagleTimer 0.0))
  (:Released
    (Transformation|SetWorldScale3D _staticmesh "0.500000,0.500000,0.500000")
    (Character|LaunchCharacter "-154.500000, 0,250.000000" false false)
    (Audio|PlaySoundatLocation "/Game/Cluck_Cue.Cluck_Cue" "0, 0, 0" "0, 0, 0" 1.0 1.0 0.0 0 0 0)
    (Transformation|AddWorldOffset (Variables|Default|GetCamera) "10.000000, 0, 0" false false)))

(fn ConstructionScript)

(fn SpawnEagle
  (params (SpawnLocation :type Vector))
  (Game|SpawnActorfromClass "/Game/BP_Eagle.BP_Eagle_C" (Math|Transform|MakeTransform SpawnLocation "0,90.000000, 0" "1,1,1") "Undefined" 0 0))

(fn Restart
  (bind _returnvalue (Game|GetPlayerController 0))
  (bind _outactors (Actor|GetAllActorsOfClass "/Game/BP_Coin.BP_Coin_C"))
  (for _array_element _outactors
    (Actor|DestroyActor _array_element))
  (bind _outactors_2 (Actor|GetAllActorsOfClass "/Game/BP_LTree.BP_LTree_C"))
  (for _array_element_2 _outactors_2
    (Actor|DestroyActor _array_element_2))
  (bind _outactors_3 (Actor|GetAllActorsOfClass "/Game/BP_MTree.BP_MTree_C"))
  (for _array_element_3 _outactors_3
    (Actor|DestroyActor _array_element_3))
  (bind _outactors_4 (Actor|GetAllActorsOfClass "/Game/BP_STree.BP_STree_C"))
  (for _array_element_4 _outactors_4
    (Actor|DestroyActor _array_element_4))
  (bind _outactors_5 (Actor|GetAllActorsOfClass "/Game/BP_LRock.BP_LRock_C"))
  (for _array_element_5 _outactors_5
    (Actor|DestroyActor _array_element_5))
  (bind _outactors_6 (Actor|GetAllActorsOfClass "/Game/BP_MRock.BP_MRock_C"))
  (for _array_element_6 _outactors_6
    (Actor|DestroyActor _array_element_6))
  (bind _outactors_7 (Actor|GetAllActorsOfClass "/Game/BP_SRock.BP_SRock_C"))
  (for _array_element_7 _outactors_7
    (Actor|DestroyActor _array_element_7))
  (bind _outactors_8 (Actor|GetAllActorsOfClass "/Game/BP_RRCrossing.BP_RRCrossing_C"))
  (for _array_element_8 _outactors_8
    (Actor|DestroyActor _array_element_8))
  (bind _outactors_9 (Actor|GetAllActorsOfClass "/Game/BP_Car.BP_Car_C"))
  (for _array_element_9 _outactors_9
    (Actor|DestroyActor _array_element_9))
  (bind _outactors_10 (Actor|GetAllActorsOfClass "/Game/BP_Truck.BP_Truck_C"))
  (for _array_element_10 _outactors_10
    (Actor|DestroyActor _array_element_10))
  (bind _outactors_11 (Actor|GetAllActorsOfClass "/Game/BP_Police.BP_Police_C"))
  (for _array_element_11 _outactors_11
    (Actor|DestroyActor _array_element_11))
  (bind _outactors_12 (Actor|GetAllActorsOfClass "/Game/BP_Train.BP_Train_C"))
  (for _array_element_12 _outactors_12
    (Actor|DestroyActor _array_element_12))
  (bind _outactors_13 (Actor|GetAllActorsOfClass "/Game/BP_Lily.BP_Lily_C"))
  (for _array_element_13 _outactors_13
    (Actor|DestroyActor _array_element_13))
  (bind _outactors_14 (Actor|GetAllActorsOfClass "/Game/BP_Log.BP_Log_C"))
  (for _array_element_14 _outactors_14
    (Actor|DestroyActor _array_element_14))
  (Widget|RemovefromParent (Variables|Default|GetRestartHUD))
  (Input|SetInputModeGameOnly _returnvalue)
  (Variables|/Script/Engine.PlayerController|SetbShowMouseCursor _returnvalue false)
  (Variables|Default|SetCoinsCollected 0)
  (Default|UpdateCoinText (Variables|Default|GetCoinHUD))
  (Variables|Default|SeteagleTimer 0.0)
  (Transformation|SetWorldTransform (Variables|Default|GetStaticMesh) (Math|Transform|MakeTransform "0, 0,20.000000" "0, 0, 0" "0.500000,0.500000,0.500000") false false))

(fn DisplayGameOver
  (bind _returnvalue (Game|GetPlayerController 0))
  (UserInterface|Viewport|AddtoViewport (Variables|Default|GetRestartHUD) 0)
  (Input|SetInputModeUIOnly _returnvalue 0 "DoNotLock")
  (Variables|/Script/Engine.PlayerController|SetbShowMouseCursor _returnvalue true)
  (Audio|PlaySoundatLocation "/Game/GameOverSFX_Cue.GameOverSFX_Cue" "0, 0, 0" "0, 0, 0" 1.0 1.0 0.0 0 0 0))