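; BP_Police is a moving police hazard that ends the game when it hits BP_Player.
; Tick moves it along world Y, scaled by PoliceSpeed, delta time and the forward vector's X, and swaps blue and red light intensities on a frame counter.
; Three collision overlaps squash the player's mesh, vertically for PoliceBox or along X for the other two, then call DisplayGameOver and destroy the police actor.
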(event OnComponentBeginOverlap(PoliceBox)
  (params (OverlappedComponent :type Primitive%20Component%20Object%20Reference) (OtherActor :type Actor%20Object%20Reference) (OtherComp :type Primitive%20Component%20Object%20Reference) (OtherBodyIndex :type Integer) (bFromSweep :type Boolean) (SweepResult :type Hit%20Result%20Structure%20%28by%20ref%29))
  (bind _asbp_player (Utilities|Casting|CastToBP_Player OtherActor))
  (Transformation|SetWorldTransform (Variables|/Game/BP_Player.BP_Player_C|GetStaticMesh _asbp_player) (Math|Transform|MakeTransform (- (Transformation|GetWorldLocation (Variables|/Script/Engine.Actor|GetRootComponent _asbp_player)) "0, 0,5.000000") "0, 0, 0" "0.500000,0.500000,0.100000") false false)
  (Default|DisplayGameOver _asbp_player)
  (Actor|DestroyActor))

(event OnComponentBeginOverlap(PoliceCollision1)
  (params (OverlappedComponent :type Primitive%20Component%20Object%20Reference) (OtherActor :type Actor%20Object%20Reference) (OtherComp :type Primitive%20Component%20Object%20Reference) (OtherBodyIndex :type Integer) (bFromSweep :type Boolean) (SweepResult :type Hit%20Result%20Structure%20%28by%20ref%29))
  (bind _asbp_player (Utilities|Casting|CastToBP_Player OtherActor))
  (Transformation|SetWorldTransform (Variables|/Game/BP_Player.BP_Player_C|GetStaticMesh _asbp_player) (Math|Transform|MakeTransform (Transformation|GetWorldLocation (Variables|/Script/Engine.Actor|GetRootComponent _asbp_player)) "0, 0, 0" "0.100000,0.500000,0.500000") false false)
  (Default|DisplayGameOver _asbp_player)
  (Actor|DestroyActor))

(event OnComponentBeginOverlap(PoliceCollision2)
  (params (OverlappedComponent :type Primitive%20Component%20Object%20Reference) (OtherActor :type Actor%20Object%20Reference) (OtherComp :type Primitive%20Component%20Object%20Reference) (OtherBodyIndex :type Integer) (bFromSweep :type Boolean) (SweepResult :type Hit%20Result%20Structure%20%28by%20ref%29))
  (bind _asbp_player (Utilities|Casting|CastToBP_Player OtherActor))
  (Transformation|SetWorldTransform (Variables|/Game/BP_Player.BP_Player_C|GetStaticMesh _asbp_player) (Math|Transform|MakeTransform (Transformation|GetWorldLocation (Variables|/Script/Engine.Actor|GetRootComponent _asbp_player)) "0, 0, 0" "0.100000,0.500000,0.500000") false false)
  (Default|DisplayGameOver _asbp_player)
  (Actor|DestroyActor))

(event EventBeginPlay)

(event Collision|EventActorBeginOverlap
  (params (OtherActor :type Actor%20Object%20Reference)))

(event EventTick
  (params (DeltaSeconds :type Float%20%28single-precision%29))
  (Transformation|AddActorWorldOffset (Math|Vector|MakeVector 0.0 (* (* DeltaSeconds (Variables|Default|GetpoliceSpeed)) (.x (Transformation|GetActorForwardVector))) 0.0))
  (Math|Integer|IncrementInt (Variables|Default|Getcount)
    (:%20%20
      (if (== (Variables|Default|Getcount) 50)
        (if (== (Variables|/Script/Engine.LightComponentBase|GetIntensity (Variables|Default|GetBlueLight)) 0.0)
          (Rendering|Components|Light|SetIntensity (Variables|Default|GetBlueLight) 1e+04)
          (Rendering|Components|Light|SetIntensity (Variables|Default|GetRedLight) 0.0)
          (Variables|Default|Setcount 0)
          (else
            (Rendering|Components|Light|SetIntensity (Variables|Default|GetBlueLight) 0.0)
            (Rendering|Components|Light|SetIntensity (Variables|Default|GetRedLight) 1e+04)
            (Variables|Default|Setcount 0)))))))

(fn ConstructionScript)